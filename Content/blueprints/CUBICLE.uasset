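; Cubicle actor that fills itself with random props and then drifts endlessly through space.
; On BeginPlay it spawns roughly as many actors as Contents has entries, picking classes at random with grid-stepped positions and random yaw.
; Valid spawns attach to Floor with location snapped to it and rotation kept relative.
; A latent MoveComponentTo loop then glides the root to successive random relative locations over long random durations.
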(event EventBeginPlay
  (bind _returnvalue (Math|Random|RandomUnitVector))
  (bind _contents (Variables|Default|Getcontents))
  (bind _floor (Variables|Default|GetFloor))
  (bind _returnvalue_2 (Utilities|Array|Length _contents))
  (bind (_x _y _z) (Math|Vector|BreakVector _returnvalue))
  (bind _returnvalue_3 (Transformation|GetWorldLocation _floor))
  ;[1 1 1] Spawn Cubicle things
  (Variables|Default|SetmaxSpawn (Math|Random|RandomIntegerinRange (- _returnvalue_2 2) (+ _returnvalue_2 2)))
  (while (> (Variables|Default|GetmaxSpawn) (Variables|Default|GetspawnIndex))
    (Variables|Default|SetspawnIndex (+ (Variables|Default|GetspawnIndex) 1))
    (bind _returnvalue_4 (Game|SpawnActorfromClass (Utilities|Array|Get(acopy) _contents (Math|Random|RandomIntegerinRange 0 _returnvalue_2)) (Math|Transform|MakeTransform (Math|Vector|MakeVector (+ (.x _returnvalue_3) (Math|Conversions|ToFloat(Integer) (- (* (Math|Random|RandomIntegerinRange 0 4) 250) 500))) (+ (.y _returnvalue_3) (Math|Conversions|ToFloat(Integer) (- (* (Math|Random|RandomIntegerinRange 0 4) 250) 500))) (+ (.z _returnvalue_3) 5e+01)) (Math|Rotator|MakeRotator 0.0 0.0 (Math|Random|RandomFloatinRange 0.0 3.6e+02))) "Undefined" 0 0))
    (if (Utilities|IsValid _returnvalue_4)
      (Transformation|AttachComponentToComponent _returnvalue_4 (Variables|Default|GetFloor) "None" "SnapToTarget" "KeepRelative" "KeepRelative" true)))
  (Variables|Default|SetspawnIndex 0)
  ;[1 1 1] Move the Cubicle
  (Components|MoveComponentTo (Variables|Default|GetDefaultSceneRoot) (Math|Vector|MakeVector (- (* _x 1e+04) 1e+04) (- (* _y 2e+04) 1e+04) (- (* _z 2e+03) 1e+03)) "0, 0, 0" false false (+ (* (Math|Random|RandomFloat) 1.2e+02) 3e+01) :!label _label)
  (Utilities|FlowControl|Delay 0.1)
  (goto _label))

(fn ConstructionScript)